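; Turret enemy pawn Blueprint that handles the loot dropped when the turret is destroyed.
; HandleDestruction always drops an experience pickup under the BP_GMLevelUp game mode.
; In other modes a coin flip gates the drop, then weighted rolls choose time, health or a random PickupsArray entry via SpawnPickup, offset slightly from the turret.
; Every path ends by destroying the actor.
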(event `self.ReceiveBeginPlay`)

(event `self.ReceiveTick`
  (params (DeltaSeconds :type "Float (single-precision)")))

(event `self.HandleDestruction`
  (bind (_returnvalue_x _returnvalue_y _returnvalue_z) (`KismetMathLibrary.BreakVector` (`self.K2_GetActorLocation`)))
  (bind (_returnvalue_location _returnvalue_rotation _returnvalue_scale) (`KismetMathLibrary.BreakTransform` (`self.GetTransform`)))
  (bind (_returnvalue_x_2 _returnvalue_y_2 _returnvalue_z_2) (`KismetMathLibrary.BreakVector` (`self.K2_GetActorLocation`)))
  (`/Engine/EditorBlueprintResources/StandardMacros.IsValid` (cast `/Game/Blueprints/BP_GMLevelUp` (`GameplayStatics.GetGameMode`) :!pure true)
    (:`Is Valid`
      (`|SpawnActorFromClass` "/Game/Blueprints/Pickups/BP_PickupExp.BP_PickupExp_C" (`KismetMathLibrary.MakeTransform` _returnvalue_location _returnvalue_rotation _returnvalue_scale) "AlwaysSpawn" "OverrideRootScale" null null)
      (`self.K2_DestroyActor` :!label _label))
    (:`Is Not Valid`
      (if (`KismetMathLibrary.RandomBool`)
        (if (>= (`KismetMathLibrary.RandomInteger` 5) 4)
          (`self.SpawnPickup`)
          (elif (<= (`KismetMathLibrary.RandomInteger` 5) 2)
            (`|SpawnActorFromClass` "/Game/Blueprints/Pickups/BP_PickupTime.BP_PickupTime_C" (`KismetMathLibrary.MakeTransform` (`KismetMathLibrary.MakeVector` (+ (`KismetMathLibrary.RandomFloatInRange` 50.0 100.0) _returnvalue_x) (+ (`KismetMathLibrary.RandomFloatInRange` 50.0 100.0) _returnvalue_y) _returnvalue_z)) "AlwaysSpawn" "OverrideRootScale" null null)
            (else
              (`|SpawnActorFromClass` "/Game/Blueprints/Pickups/BP_PickupHealth.BP_PickupHealth_C" (`KismetMathLibrary.MakeTransform` (`KismetMathLibrary.MakeVector` (+ (`KismetMathLibrary.RandomFloatInRange` 50.0 100.0) _returnvalue_x_2) (+ (`KismetMathLibrary.RandomFloatInRange` 50.0 100.0) _returnvalue_y_2) _returnvalue_z_2)) "AlwaysSpawn" "OverrideRootScale" null null))))
        (`self.K2_DestroyActor`)
        (else
          (goto _label))))))

(fn `SpawnPickup`
  (bind (_returnvalue_x _returnvalue_y _returnvalue_z) (`KismetMathLibrary.BreakVector` (`self.K2_GetActorLocation`)))
  (`|SpawnActorFromClass` (`KismetArrayLibrary.Array_Random` (`self.PickupsArray`)) (`KismetMathLibrary.MakeTransform` (`KismetMathLibrary.MakeVector` (+ (`KismetMathLibrary.RandomFloatInRange` 50.0 100.0) _returnvalue_x) (+ (`KismetMathLibrary.RandomFloatInRange` 50.0 100.0) _returnvalue_y) _returnvalue_z)) "AlwaysSpawn" "OverrideRootScale" null null))

(fn `UserConstructionScript`)